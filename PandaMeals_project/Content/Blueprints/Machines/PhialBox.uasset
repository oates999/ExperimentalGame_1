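; PhialBox is a clickable dispenser that spawns a Phial of its configured MeatType already attached to the cursor.
; Tick polls cursor hover and the Player_Pawn's left-mouse state to set a transient attach flag, which spawns the Phial and clears only while the box is Enabled.
; UpdateImage, not called within this Blueprint, dims the sprite when disabled and sets its sort priority from Layer.
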(event Custom|Update%20Image
  (if (Variables|Default|Getenabled)
    (Sprite|SetSpriteColor (Variables|Default|GetBoxImage) "(R=1.000000,G=1.000000,B=1.000000,A=1.000000)")
    (else
      (Sprite|SetSpriteColor (Variables|Default|GetBoxImage) "(R=0.317708,G=0.317708,B=0.317708,A=1.000000)")))
  (Rendering|SetTranslucentSortPriority (Variables|Default|GetBoxImage) (* (Variables|Default|Getlayer) 100)))

(event Custom|Check%20Attach
  (bind _player (Variables|Default|Getplayer))
  (bind _cursor_hover (Variables|Default|Getcursor_hover))
  (bind _attached_to_cursor (Variables|Default|Getattached_to_cursor))
  (bind _returnvalue (not _attached_to_cursor))
  (bind _lmb_down (Variables|/Game/Blueprints/Player_Pawn.Player_Pawn_C|Getlmb_down _player))
  (bind _returnvalue_2 (Math|Boolean|ANDBoolean _cursor_hover _lmb_down _returnvalue))
  (if _returnvalue_2
    (CallFunction|SetAttached _returnvalue_2)))

(event Custom|Set%20Attached
  (params (attached :type Boolean))
  (Variables|Default|Setattached_to_cursor attached))

(event Custom|Pick%20Up
  (if (Variables|Default|Getattached_to_cursor)
    (if (Variables|Default|Getenabled)
      (bind _returnvalue (Game|SpawnActorfromClass "/Game/Blueprints/Objects/Phial.Phial_C" (Transformation|GetWorldTransform (Variables|Default|GetDefaultSceneRoot)) "Undefined" 0 0))
      (Rendering|SetTranslucentSortPriority (Variables|/Game/Blueprints/Objects/Phial.Phial_C|GetPhialImage _returnvalue) 10000)
      (Default|Constructor:MeatOfType _returnvalue (Variables|Default|Getmeat_type))
      (Default|SetAttached _returnvalue true)
      (CallFunction|SetAttached false))))

(event EventBeginPlay
  (bind _asplayer_pawn (Utilities|Casting|CastToPlayer_Pawn (Pawn|GetControlledPawn (Game|GetPlayerController 0))))
  (Variables|Default|Setplayer _asplayer_pawn))

(event EventTick
  (params (DeltaSeconds :type Float%20%28single-precision%29))
  (CallFunction|CheckAttach)
  (CallFunction|PickUp))

(event MouseInput|EventActorBeginCursorOver
  (Variables|Default|Setcursor_hover true))

(event MouseInput|EventActorEndCursorOver
  (Variables|Default|Setcursor_hover false))

(fn ConstructionScript)