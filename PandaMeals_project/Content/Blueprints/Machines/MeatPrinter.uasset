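; Meat printer machine actor that produces packaged meat of a requested type.
; PrintMeat marks the printer busy, shows the meat type's icon and starts a fixed timer.
; When the timer ends, it clears the icon, spawns and initialises a PackagedMeat at the printer and adds it to the packaged meat manager's queue.
; BeginPlay derives the sprites' translucent sort priorities from the printer's layer.
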(event Custom|Print%20Meat
  (params (meat_type :type String))
  (Variables|Default|Setis_ready false)
  (Variables|Default|Setcurrent_meat meat_type)
  (Rendering|Components|Sprite|SetSprite (Variables|Default|GetIconImage) (.Value (Utilities|Map|Find (Variables|Default|Getmeat_images) meat_type)))
  (Utilities|Time|SetTimerbyFunctionName 0 "Finish Print" 3.0))

(event Custom|Finish%20Print
  (bind _packagedmeat_manager (Variables|Default|Getpackagedmeat_manager))
  (Variables|Default|Setis_ready true)
  (bind _returnvalue (Game|SpawnActorfromClass "/Game/Blueprints/Objects/PackagedMeat.PackagedMeat_C" (Transformation|GetWorldTransform (Variables|Default|GetDefaultSceneRoot)) "Undefined" 0 0))
  (Rendering|SetTranslucentSortPriority (Variables|/Game/Blueprints/Objects/PackagedMeat.PackagedMeat_C|GetPackagedMeatImage _returnvalue) 10000)
  (Rendering|Components|Sprite|SetSprite (Variables|Default|GetIconImage) 0)
  (Default|Constructor:MeatOfType _returnvalue (Variables|Default|Getcurrent_meat) _packagedmeat_manager)
  (Default|AddMeattoQueue _packagedmeat_manager _returnvalue))

(event EventBeginPlay
  (bind _layer (Variables|Default|Getlayer))
  (bind _returnvalue (* _layer 100))
  ;[1 1 1] Comment
  (Rendering|SetTranslucentSortPriority (Variables|Default|GetMeatPrinterImager_Back) _returnvalue)
  (Rendering|SetTranslucentSortPriority (Variables|Default|GetMeatPrinterImage) (+ _returnvalue 1))
  (Rendering|SetTranslucentSortPriority (Variables|Default|GetIconImage) (+ _returnvalue 2)))

(fn ConstructionScript)