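; PaperBag is a machine that collects up to three ingredients and checks them against the first order in OrderManager.
; AddIngredient shows each item's sprite from MeatSprites, layers bag and ingredient sprites by translucent sort priority, then runs CheckComplete.
; CheckComplete compares contents regardless of order by removing matches from a temporary copy.
; A match fulfills the order and clears the bag; a full bag without a match is also cleared.
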(event Custom|Add%20Ingredient
  (params (added_ingredient :type String))
  (bind _ingredients (Variables|Default|Getingredients))
  (Utilities|Array|Add _ingredients added_ingredient)
  (for (_array_element _array_index) _ingredients
    (if (== _array_index 0)
      (Rendering|Components|Sprite|SetSprite (Variables|Default|GetIngr1Image) (.Value (Utilities|Map|Find (Variables|Default|Getmeat_sprites) _array_element)))
      (elif (== _array_index 1)
        (Rendering|Components|Sprite|SetSprite (Variables|Default|GetIngr2Image) (.Value (Utilities|Map|Find (Variables|Default|Getmeat_sprites) _array_element)))
        (elif (== _array_index 2)
          (Rendering|Components|Sprite|SetSprite (Variables|Default|GetIngr3Image) (.Value (Utilities|Map|Find (Variables|Default|Getmeat_sprites) _array_element)))))))
  (CallFunction|SetY-AxisValues)
  (CallFunction|CheckComplete))

(event Custom|Set%20Y-Axis%20Values
  (bind _layer (Variables|Default|Getlayer))
  (bind _returnvalue (* _layer 100))
  (bind _returnvalue_2 (+ _returnvalue 1))
  (bind _returnvalue_3 (+ _returnvalue_2 1))
  (Rendering|SetTranslucentSortPriority (Variables|Default|GetBagImage) _returnvalue)
  (Rendering|SetTranslucentSortPriority (Variables|Default|GetIngr1Image) _returnvalue_2)
  (Rendering|SetTranslucentSortPriority (Variables|Default|GetIngr2Image) _returnvalue_3)
  (Rendering|SetTranslucentSortPriority (Variables|Default|GetIngr3Image) (+ _returnvalue_3 1)))

(event Custom|Check%20Complete
  (bind _order_manager (Variables|Default|Getorder_manager))
  (bind _orders (Variables|/Game/Blueprints/Managers/Order_Manager.Order_Manager_C|Getorders _order_manager))
  (bind _output (Utilities|Array|Get(acopy) _orders))
  (bind _ingredients (Variables|/Game/Blueprints/Objects/Order.Order_C|Getingredients _output))
  (Variables|Default|Settemp (Variables|Default|Getingredients))
  (if (== (Utilities|Array|Length (Variables|Default|Getingredients)) (Utilities|Array|Length _ingredients))
    (for _array_element _ingredients
      (if (!= (Utilities|Array|FindItem (Variables|Default|Gettemp) _array_element) -1)
        (Utilities|Array|RemoveIndex (Variables|Default|Gettemp) (Utilities|Array|FindItem (Variables|Default|Gettemp) _array_element))))
    (if (== (Utilities|Array|Length (Variables|Default|Gettemp)) 0)
      (Default|FulfillFirstOrder _order_manager)
      (CallFunction|ClearBag)
      (else
        (if (== (Utilities|Array|Length (Variables|Default|Getingredients)) 3) :!label _label
          (CallFunction|ClearBag))))
    (else
      (goto _label))))

(event Custom|Clear%20Bag
  (Utilities|Array|Clear (Variables|Default|Getingredients))
  (Rendering|Components|Sprite|SetSprite (Variables|Default|GetIngr1Image) 0)
  (Rendering|Components|Sprite|SetSprite (Variables|Default|GetIngr2Image) 0)
  (Rendering|Components|Sprite|SetSprite (Variables|Default|GetIngr3Image) 0)
  (Utilities|Array|Clear (Variables|Default|Gettemp))
  (Variables|Default|Setcounter 0))

(event EventBeginPlay
  (CallFunction|ClearBag)
  (CallFunction|SetY-AxisValues))

(fn ConstructionScript)