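; Splicer machine actor that turns a given meat type into a new petri dish after a timed splice.
; On BeginPlay it layers its machine and icon sprites by translucent sort priority.
; SpliceMeat marks it busy, shows the meat's icon and starts a three-second timer.
; Finish Splice frees it, clears the icon, spawns a petri dish of that meat and queues it with the splicer's petri dish manager.
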(event Custom|Splice%20Meat
  (params (meat_type :type String))
  (Variables|Default|Setis_ready false)
  (Variables|Default|Setcurrent_meat meat_type)
  (Rendering|Components|Sprite|SetSprite (Variables|Default|GetIconImage) (.Value (Utilities|Map|Find (Variables|Default|Getmeat_images) meat_type)))
  (Utilities|Time|SetTimerbyFunctionName 0 "Finish Splice" 3.0))

(event Custom|Finish%20Splice
  (bind _petridish_manager_splicer (Variables|Default|Getpetridish_manager_splicer))
  (Variables|Default|Setis_ready true)
  (bind _returnvalue (Game|SpawnActorfromClass "/Game/Blueprints/Objects/PetriDish.PetriDish_C" (Transformation|GetWorldTransform (Variables|Default|GetDefaultSceneRoot)) "Undefined" 0 0))
  (Rendering|SetTranslucentSortPriority (Variables|/Game/Blueprints/Objects/PetriDish.PetriDish_C|GetPetriDishImage _returnvalue) 10000)
  (Default|Constructor:MeatOfType _returnvalue (Variables|Default|Getcurrent_meat) _petridish_manager_splicer (Variables|/Game/Blueprints/Managers/PetriDish_Manager_Splicer.PetriDish_Manager_Splicer_C|Getprinter_manager _petridish_manager_splicer))
  (Variables|/Game/Blueprints/Objects/PetriDish.PetriDish_C|Setin_splicer _returnvalue true)
  (Rendering|Components|Sprite|SetSprite (Variables|Default|GetIconImage) 0)
  (Default|AddPetriDishtoQueue (Variables|Default|Getpetridish_manager_splicer) _returnvalue))

(event EventBeginPlay
  (bind _layer (Variables|Default|Getlayer))
  (bind _returnvalue (* _layer 100))
  ;[1 1 1] Comment
  (Rendering|SetTranslucentSortPriority (Variables|Default|GetSplicerImage) _returnvalue)
  (Rendering|SetTranslucentSortPriority (Variables|Default|GetIconImage) (+ _returnvalue 1)))

(fn ConstructionScript)