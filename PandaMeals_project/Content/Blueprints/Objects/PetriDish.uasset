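; Draggable petri dish actor that holds one meat type, shows its matching sprite and moves between the splicer, printer and trash.
; Tick checks for left-click on hover, removes the dish from its current manager, then snaps it to a mouse line trace.
; Overlapping trash destroys it.
; Overlapping a meat printer while held spawns a replacement copy into that printer's queue and destroys the original.
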(event OnComponentBeginOverlap(PetriDishImage)
  (params (OverlappedComponent :type Primitive%20Component%20Object%20Reference) (OtherActor :type Actor%20Object%20Reference) (OtherComp :type Primitive%20Component%20Object%20Reference) (OtherBodyIndex :type Integer) (bFromSweep :type Boolean) (SweepResult :type Hit%20Result%20Structure%20%28by%20ref%29))
  (Utilities|Casting|CastToTrash OtherActor
    (:then
      (CallFunction|Destructor:EnterPrinter))
    (:CastFailed
      (bind _asmeat_printer (Utilities|Casting|CastToMeatPrinter OtherActor))
      (if (Variables|Default|Getattached_to_cursor)
        (bind _returnvalue (Game|SpawnActorfromClass "PetriDish_C" (Transformation|GetWorldTransform (Variables|Default|GetDefaultSceneRoot)) "Undefined" 0 0))
        (CallFunction|Constructor:MeatOfType _returnvalue (Variables|Default|Getmeat_type) (Variables|Default|Getsplicer_manager) (Variables|Default|Getprinter_manager))
        (Default|AddPetriDishtoQueue (Variables|/Game/Blueprints/Machines/MeatPrinter.MeatPrinter_C|Getpetridish_manager_printer _asmeat_printer) _returnvalue)
        (Variables|Default|Setattached_to_cursor false)
        (Variables|PetriDish_C|Setin_printer _returnvalue true)
        (Variables|PetriDish_C|Setin_splicer _returnvalue false)
        (Actor|DestroyActor)))))

(event Custom|Constructor:%20Meat%20of%20Type
  (params (meat_type :type String) (splicer_manager :type Petri%20Dish%20Manager%20Splicer%20Object%20Reference) (printer_manager :type Petri%20Dish%20Manager%20Printer%20Object%20Reference))
  (Variables|Default|Setprinter_manager printer_manager)
  (Variables|Default|Setsplicer_manager splicer_manager)
  (bind _output_get (Variables|Default|Setmeat_type meat_type))
  (if (.ReturnValue (Utilities|Map|Find (Variables|Default|Getpetri_sprites) _output_get))
    (Rendering|Components|Sprite|SetSprite (Variables|Default|GetPetriDishImage) (.Value (Utilities|Map|Find (Variables|Default|Getpetri_sprites) _output_get)))
    (else
      (Development|PrintString "Ingredient not found!"))))

(event Custom|Destructor:%20Enter%20Printer
  ;[1 0 0.79] PLACEHOLDER
  (Actor|SetLifeSpan 0.1))

(event Custom|Check%20Attach
  (if (Math|Boolean|ANDBoolean (Variables|Default|Getcursor_hover) (Variables|/Game/Blueprints/Player_Pawn.Player_Pawn_C|Getlmb_down (Variables|Default|Getplayer)) (not (Variables|Default|Getattached_to_cursor)))
    (CallFunction|SetAttached true)
    (if (Variables|Default|Getin_printer)
      (Default|RemovePetriDish (Variables|Default|Getprinter_manager) self)
      (else
        (Default|RemovePetriDish (Variables|Default|Getsplicer_manager) self)))))

(event Custom|Set%20Attached
  (params (attached :type Boolean))
  (Variables|Default|Setattached_to_cursor attached))

(event Custom|Pick%20Up
  (bind _returnvalue (Game|GetPlayerController 0))
  (bind (_worldlocation _worlddirection) (Game|Player|ConvertMouseLocationToWorldSpace _returnvalue))
  (if (Variables|Default|Getattached_to_cursor)
    (bind (_outhit _returnvalue_2) (Collision|LineTraceByChannel _worldlocation (+ _worldlocation (* _worlddirection 2e+03)) "TraceTypeQuery3" false 0 "None"))
    (if _returnvalue_2
      (Transformation|SetActorLocation (+ (.Location (Collision|BreakHitResult _outhit)) "0,10.000000,0.000000") false true))))

(event EventBeginPlay
  (bind _asplayer_pawn (Utilities|Casting|CastToPlayer_Pawn (Pawn|GetControlledPawn (Game|GetPlayerController 0))))
  (Variables|Default|Setplayer _asplayer_pawn))

(event EventTick
  (params (DeltaSeconds :type Float%20%28single-precision%29))
  (CallFunction|CheckAttach)
  (CallFunction|PickUp))

(event MouseInput|EventActorBeginCursorOver
  (Variables|Default|Setcursor_hover true))

(event MouseInput|EventActorEndCursorOver
  (Variables|Default|Setcursor_hover false))

(fn ConstructionScript)