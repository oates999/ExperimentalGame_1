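; Phial manager that keeps a spaced queue of meat phials feeding a Splicer, pre-filled at BeginPlay with "panda" phials.
; A small random chance each tick passes the front phial's meat type to the Splicer and removes that phial.
; The rest temporarily attach to PhialMover, which a timeline slides one slot forward, then detach and get slight Y staggering against Z-fighting.
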(event Custom|Add%20Phial%20to%20Queue
  (params (added_phial :type Phial%20Object%20Reference))
  (bind _defaultsceneroot (Variables|Default|GetDefaultSceneRoot))
  (bind _returnvalue (Transformation|GetWorldLocation _defaultsceneroot))
  (Transformation|SetActorLocation added_phial (Math|Vector|MakeVector (+ (.x _returnvalue) (* -1 (* (Utilities|Array|Length (Variables|Default|Getphials)) (Variables|Default|Getphial_offset)))) (.y _returnvalue) (.z _returnvalue)) false true)
  (Utilities|Array|Add (Variables|Default|Getphials) added_phial))

(event Custom|Send%20First%20Phial%20to%20Splicer
  ;[0.4314 0.4314 0.4314] Sends first phial to splicer and removes it.
  (Default|SpliceMeat (Variables|Default|Getsplicer) (Variables|/Game/Blueprints/Objects/Phial.Phial_C|Getmeat_type (Utilities|Array|Get(acopy) (Variables|Default|Getphials))))
  (Default|Destructor:EnterSplicer (Utilities|Array|Get(acopy) (Variables|Default|Getphials)))
  (Utilities|Array|RemoveIndex (Variables|Default|Getphials))
  (Transformation|SetRelativeLocation (Variables|Default|GetPhialMover) "0, 0, 0" false true)
  (for _array_element (Variables|Default|Getphials)
    (Transformation|AttachComponentToComponent _array_element (Variables|Default|GetPhialMover) "None" "KeepWorld" "KeepWorld" "KeepWorld" false))
  (bind _spline__0_to_1_ (Timeline|Phial%20Mover%20Mover PlayFromStart)
    (:Update
      (Transformation|SetRelativeLocation (Variables|Default|GetPhialMover) (Math|Vector|MakeVector (* _spline__0_to_1_ (Variables|Default|Getphial_offset)) 0.0 0.0) false true))
    (:Finished
      (for _array_element_2 (Variables|Default|Getphials)
        (Transformation|DetachFromActor _array_element_2 "KeepWorld" "KeepWorld" "KeepWorld"))
      (CallFunction|SetY-AxisValues))))

(event Custom|Set%20Y-Axis%20Values
  (bind _phials (Variables|Default|Getphials))
  ;[0.4314 0.4314 0.4314] Sets phial relative locations (Y axis) to prevent Z-fighting
  (for (_array_element _array_index) _phials
    (Transformation|SetActorRelativeLocation _array_element (Math|Vector|MakeVector (.x (Transformation|GetActorLocation _array_element)) (+ (.y (Transformation|GetActorLocation (Utilities|Array|Get(acopy) _phials))) (* _array_index -0.1)) (.z (Transformation|GetActorLocation _array_element))) false true)))

(event EventTick
  (params (DeltaSeconds :type Float%20%28single-precision%29))
  (if (> (Math|Random|RandomFloatinRange 0.0 1e+02) 99.9)
    (CallFunction|SendFirstPhialtoSplicer)))

(event EventBeginPlay
  (while (<= (Utilities|Array|Length (Variables|Default|Getphials)) (Variables|Default|Getmax_size))
    (bind _returnvalue (Game|SpawnActorfromClass "/Game/Blueprints/Objects/Phial.Phial_C" (Transformation|GetWorldTransform (Variables|Default|GetDefaultSceneRoot)) "Undefined" 0 0))
    (Default|Constructor:MeatOfType _returnvalue "panda")
    (CallFunction|AddPhialtoQueue _returnvalue)))

(fn ConstructionScript)