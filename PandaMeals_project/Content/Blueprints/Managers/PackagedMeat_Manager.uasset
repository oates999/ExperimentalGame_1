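; Manager actor for a belt of packaged meat, animating the queue as items are added or removed.
; Meat is temporarily attached to the MeatMover component, which a timeline slides by an offset: all items along X on add, those after the removed one along Z on removal.
; When each slide finishes, it detaches items, reassigns translucent sort priorities by index and layer to avoid Z-fighting, and refreshes their manager references.
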(event Custom|Set%20Y-Axis%20Values
  ;[0.4314 0.4314 0.4314] Sets order relative locations (Y axis) to prevent Z-fighting
  (for (_array_element _array_index) (Variables|Default|Getpackaged_meat)
    (Rendering|SetTranslucentSortPriority (Variables|/Game/Blueprints/Objects/PackagedMeat.PackagedMeat_C|GetPackagedMeatImage _array_element) (+ _array_index (* (Variables|Default|Getlayer) 100)))))

(event Custom|Fix%20References%20in%20Array
  ;[0.4314 0.4314 0.4314] Makes sure all entries in array have correct references
  (for _array_element (Variables|Default|Getpackaged_meat)
    (Variables|/Game/Blueprints/Objects/PackagedMeat.PackagedMeat_C|Setmeat_manager _array_element self)))

(event Custom|Add%20Meat%20to%20Queue
  (params (added_meat :type Packaged%20Meat%20Object%20Reference))
  ;[0.4314 0.4314 0.4314] Adds packaged meat to the queue and advances the queue forward a step
  (Transformation|SetActorRelativeLocation added_meat (Math|Vector|MakeVector 0.0 0.0 0.0) false true)
  (Utilities|Array|Add (Variables|Default|Getpackaged_meat) added_meat)
  (Transformation|SetRelativeLocation (Variables|Default|GetMeatMover) "0, 0, 0" false true)
  (for _array_element (Variables|Default|Getpackaged_meat)
    (Transformation|AttachComponentToComponent _array_element (Variables|Default|GetMeatMover) "None" "KeepWorld" "KeepWorld" "KeepWorld" false))
  (bind _spline__0_to_1_ (Timeline|Meat%20Mover%20Mover PlayFromStart)
    (:Update
      (Transformation|SetRelativeLocation (Variables|Default|GetMeatMover) (Math|Vector|MakeVector (* _spline__0_to_1_ (Variables|Default|Getmeat_offset)) 0.0 0.0) false true))
    (:Finished
      (for _array_element_2 (Variables|Default|Getpackaged_meat)
        (Transformation|DetachFromActor _array_element_2 "KeepWorld" "KeepWorld" "KeepWorld"))
      (CallFunction|SetY-AxisValues)
      (CallFunction|FixReferencesinArray))))

(event Custom|Remove%20Packaged%20Meat
  (params (removed_meat :type Packaged%20Meat%20Object%20Reference))
  (bind _packaged_meat (Variables|Default|Getpackaged_meat))
  (bind _returnvalue (Utilities|Array|FindItem _packaged_meat removed_meat))
  ;[0.4314 0.4314 0.4314] Removes the n-th packaged neat from the belt
  (Transformation|SetRelativeLocation (Variables|Default|GetMeatMover) "0, 0, 0" false true)
  (for (_array_element _array_index) (Variables|Default|Getpackaged_meat)
    (if (> _array_index _returnvalue)
      (Transformation|AttachComponentToComponent (Variables|/Script/Engine.Actor|GetRootComponent _array_element) (Variables|Default|GetMeatMover) "None" "KeepWorld" "KeepWorld" "KeepWorld" false)))
  (bind _spline__0_to_1_ (Timeline|Meat%20Mover%20Mover%202 PlayFromStart)
    (:Update
      (Transformation|SetRelativeLocation (Variables|Default|GetMeatMover) (Math|Vector|MakeVector 0.0 0.0 (* _spline__0_to_1_ (Variables|Default|Getmeat_offset))) false true))
    (:Finished
      (for (_ _array_index_2) (Variables|Default|Getpackaged_meat)
        (if (> _array_index_2 _returnvalue)
          (Transformation|DetachFromActor "KeepWorld" "KeepWorld" "KeepWorld")))
      (Utilities|Array|RemoveIndex (Variables|Default|Getpackaged_meat) _returnvalue)
      (CallFunction|SetY-AxisValues)
      (CallFunction|FixReferencesinArray))))

(fn ConstructionScript)