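; Manager actor that keeps a vertical queue of petri dishes and feeds the first one's meat type to the MeatPrinter whenever it is ready.
; A looping timer checks the printer, and dishes can also be removed from anywhere in the stack.
; To close gaps, remaining dishes are temporarily attached to a PetriMover component that a timeline slides down one slot.
; Each change refreshes translucent sort priorities against Z-fighting and re-sets the dishes' manager references.
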(event Custom|Remove%20Petri%20Dish
  (params (removed_dish :type Petri%20Dish%20Object%20Reference))
  (bind _petri_dishes (Variables|Default|Getpetri_dishes))
  (bind _returnvalue (Utilities|Array|FindItem _petri_dishes removed_dish))
  ;[0.4314 0.4314 0.4314] Removes n-th petri dish from the stack
  (Transformation|SetRelativeLocation (Variables|Default|GetPetriMover) "0, 0, 0" false true)
  (for (_array_element _array_index) (Variables|Default|Getpetri_dishes)
    (if (> _array_index _returnvalue)
      (Transformation|AttachComponentToComponent (Variables|/Script/Engine.Actor|GetRootComponent _array_element) (Variables|Default|GetPetriMover) "None" "KeepWorld" "KeepWorld" "KeepWorld" false)))
  (bind _spline__0_to_1_ (Timeline|Timeline_0 PlayFromStart)
    (:Update
      (Transformation|SetRelativeLocation (Variables|Default|GetPetriMover) (Math|Vector|MakeVector 0.0 0.0 (* _spline__0_to_1_ (* -1 (Variables|Default|Getpetri_offset)))) false true))
    (:Finished
      (for (_array_element_2 _array_index_2) (Variables|Default|Getpetri_dishes)
        (if (> _array_index_2 _returnvalue)
          (Transformation|DetachFromActor _array_element_2 "KeepWorld" "KeepWorld" "KeepWorld")))
      (Utilities|Array|RemoveIndex (Variables|Default|Getpetri_dishes) _returnvalue)
      (CallFunction|SetY-AxisValues)
      (CallFunction|FixReferencesinArray))))

(event Custom|Set%20Y-Axis%20Values
  ;[0.4314 0.4314 0.4314] Sets order relative locations (Y axis) to prevent Z-fighting
  (for (_array_element _array_index) (Variables|Default|Getpetri_dishes)
    (Rendering|SetTranslucentSortPriority (Variables|/Game/Blueprints/Objects/PetriDish.PetriDish_C|GetPetriDishImage _array_element) (+ _array_index (* (Variables|Default|Getlayer) 100)))))

(event Custom|Fix%20References%20in%20Array
  ;[0.4314 0.4314 0.4314] Makes sure all entries in array have correct references
  (for _array_element (Variables|Default|Getpetri_dishes)
    (Variables|/Game/Blueprints/Objects/PetriDish.PetriDish_C|Setsplicer_manager _array_element (Variables|Default|Getsplicer_manager))
    (Variables|/Game/Blueprints/Objects/PetriDish.PetriDish_C|Setprinter_manager _array_element self)))

(event Custom|Send%20First%20PetriDish%20to%20Printer
  (bind _petri_dishes (Variables|Default|Getpetri_dishes))
  ;[0.4314 0.4314 0.4314] Sends first petri dish to printer and removes it.
  (Default|PrintMeat (Variables|Default|Getmeat_printer) (Variables|/Game/Blueprints/Objects/PetriDish.PetriDish_C|Getmeat_type (Utilities|Array|Get(acopy) (Variables|Default|Getpetri_dishes))))
  (Default|Destructor:EnterPrinter (Utilities|Array|Get(acopy) _petri_dishes))
  (Utilities|Array|RemoveIndex _petri_dishes)
  (Transformation|SetRelativeLocation (Variables|Default|GetPetriMover) "0, 0, 0" false true)
  (for _array_element (Variables|Default|Getpetri_dishes)
    (Transformation|AttachComponentToComponent (Variables|/Script/Engine.Actor|GetRootComponent _array_element) (Variables|Default|GetPetriMover) "None" "KeepWorld" "KeepWorld" "KeepWorld" false))
  (bind _spline__0_to_1_ (Timeline|Petri%20Mover%20Mover PlayFromStart)
    (:Update
      (Transformation|SetRelativeLocation (Variables|Default|GetPetriMover) (Math|Vector|MakeVector 0.0 0.0 (* _spline__0_to_1_ (* -1 (Variables|Default|Getpetri_offset)))) false true))
    (:Finished
      (for _array_element_2 (Variables|Default|Getpetri_dishes)
        (Transformation|DetachFromActor _array_element_2 "KeepWorld" "KeepWorld" "KeepWorld"))
      (CallFunction|SetY-AxisValues)
      (CallFunction|FixReferencesinArray))))

(event Custom|Check%20Dishes
  (if (and (Variables|/Game/Blueprints/Machines/MeatPrinter.MeatPrinter_C|Getis_ready (Variables|Default|Getmeat_printer)) (> (Utilities|Array|Length (Variables|Default|Getpetri_dishes)) 0))
    (CallFunction|SendFirstPetriDishtoPrinter)))

(event Custom|Add%20Petri%20Dish%20to%20Queue
  (params (petri_dish :type Petri%20Dish%20Object%20Reference))
  (bind _defaultsceneroot (Variables|Default|GetDefaultSceneRoot))
  (bind _returnvalue (Transformation|GetWorldLocation _defaultsceneroot))
  ;[0.4314 0.4314 0.4314] Adds a petri dish to the queue
  (Transformation|SetActorRelativeLocation petri_dish (Math|Vector|MakeVector (.x _returnvalue) (.y _returnvalue) (+ (* (Utilities|Array|Length (Variables|Default|Getpetri_dishes)) (Variables|Default|Getpetri_offset)) (.z _returnvalue))) false true)
  (Utilities|Array|Add (Variables|Default|Getpetri_dishes) petri_dish)
  (CallFunction|SetY-AxisValues)
  (CallFunction|FixReferencesinArray))

(event EventBeginPlay
  (Utilities|Time|SetTimerbyFunctionName 0 "Check Dishes" 1.0 true))

(fn ConstructionScript)