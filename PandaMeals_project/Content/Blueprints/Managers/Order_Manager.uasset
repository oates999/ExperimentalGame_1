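; Order manager actor that runs a row of eight hooks holding meat orders and tracks the player's money.
; SpawnOrder fills the first empty hook using MeatAvailability.
; FulfillFirstOrder adds ingredient prices from MeatPrices to CurrentMoney, removes the front order and appends an empty hook.
; The remaining hooks temporarily attach to OrderMover for a timeline slide forward, with small Y offsets to prevent Z-fighting.
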(event Custom|Fulfill%20First%20Order
  (bind _orders (Variables|Default|Getorders))
  ;[0.4314 0.4314 0.4314] Fulfills and removes the top order, increasing total money. Spawns a new empty hook
  (for _array_element (Variables|/Game/Blueprints/Objects/Order.Order_C|Getingredients (Utilities|Array|Get(acopy) (Variables|Default|Getorders)))
    (if (.ReturnValue (Utilities|Map|Find (Variables|Default|Getmeat_prices) _array_element))
      (Variables|Default|Setcurrent_money (+ (Variables|Default|Getcurrent_money) (.Value (Utilities|Map|Find (Variables|Default|Getmeat_prices) _array_element))))
      (else
        (Development|PrintString "Ingredient not found!"))))
  (bind _returnvalue (Game|SpawnActorfromClass "/Game/Blueprints/Objects/Order.Order_C" (Transformation|GetWorldTransform (Variables|Default|GetDefaultSceneRoot)) "Undefined" 0 0))
  (Default|Constructor:Hook _returnvalue)
  (Transformation|AttachActorToActor _returnvalue self "None" "SnapToTarget" "SnapToTarget" "SnapToTarget" false)
  (Transformation|SetActorRelativeLocation _returnvalue (Math|Vector|MakeVector (* -1 (* (Utilities|Array|Length (Variables|Default|Getorders)) (Variables|Default|Getorder_offset))) 0.0 0.0) false true)
  (Utilities|Array|Add _orders _returnvalue)
  (Default|Destructor:FulfillOrder (Utilities|Array|Get(acopy) _orders))
  (Utilities|Array|RemoveIndex _orders)
  (Transformation|SetRelativeLocation (Variables|Default|GetOrderMover) "0, 0, 0" false true)
  (for _array_element_2 (Variables|Default|Getorders)
    (Transformation|DetachFromActor _array_element_2 "KeepWorld" "KeepWorld" "KeepWorld")
    (Transformation|AttachComponentToComponent (Variables|/Script/Engine.Actor|GetRootComponent _array_element_2) (Variables|Default|GetOrderMover) "None" "KeepWorld" "KeepWorld" "KeepWorld" false))
  (bind _spline__0_to_1_ (Timeline|Order%20Mover%20Mover PlayFromStart)
    (:Update
      (Transformation|SetRelativeLocation (Variables|Default|GetOrderMover) (Math|Vector|MakeVector (* _spline__0_to_1_ (* 1 (Variables|Default|Getorder_offset))) 0.0 0.0) false true))
    (:Finished
      (for _array_element_3 (Variables|Default|Getorders)
        (Transformation|DetachFromActor _array_element_3 "KeepWorld" "KeepWorld" "KeepWorld")
        (Transformation|AttachActorToActor _array_element_3 self "None" "KeepWorld" "KeepWorld" "KeepWorld" false))
      (CallFunction|SetY-AxisValues))))

(event Custom|Set%20Y-Axis%20Values
  ;[0.4314 0.4314 0.4314] Sets order relative locations (Y axis) to prevent Z-fighting
  (for (_array_element _array_index) (Variables|Default|Getorders)
    (Transformation|SetActorRelativeLocation _array_element (Math|Vector|MakeVector (.x (Transformation|GetActorLocation _array_element)) (* _array_index -0.1) (.z (Transformation|GetActorLocation _array_element))) false true)))

(event Custom|Spawn%20Order
  ;[0.4314 0.4314 0.4314] Fills first empty hook with a generated order
  (bind (_array_element _array_index) (Utilities|Array|ForEachLoopwithBreak (Variables|Default|Getorders) :!label _label)
    (:LoopBody
      (if (Math|Boolean|Equal(Boolean) (Variables|/Game/Blueprints/Objects/Order.Order_C|Getempty? _array_element) true)
        (Default|Constructor:Order _array_element (Variables|Default|Getmeat_availability))
        (goto _label Break)
        (elif (== _array_index (- (Utilities|Array|Length (Variables|Default|Getorders)) 1))
          (Development|PrintString "No empty hooks!"))))
    (:Completed
      (CallFunction|SetY-AxisValues))))

(event EventTick
  (params (DeltaSeconds :type Float%20%28single-precision%29))
  (if (> (Math|Random|RandomFloatinRange 0.0 1e+02) 99.7)
    _))

(event EventBeginPlay
  (bind _orders (Variables|Default|Getorders))
  (bind _returnvalue (Utilities|Array|Length _orders))
  ;[0.4342 0.4342 0.4342] At BeginPlay, creates 8 empty hooks and adds to "orders" array
  (while (< _returnvalue 8)
    (bind _returnvalue_2 (Game|SpawnActorfromClass "/Game/Blueprints/Objects/Order.Order_C" (Transformation|GetWorldTransform (Variables|Default|GetDefaultSceneRoot)) "Undefined" 0 0))
    (Default|Constructor:Hook _returnvalue_2)
    (Transformation|AttachActorToActor _returnvalue_2 self "None" "SnapToTarget" "SnapToTarget" "SnapToTarget" false)
    (Transformation|SetActorRelativeLocation _returnvalue_2 (Math|Vector|MakeVector (* -1 (* _returnvalue (Variables|Default|Getorder_offset))) 0.0 0.0) false true)
    (Utilities|Array|Add (Variables|Default|Getorders) _returnvalue_2))
  (CallFunction|SetY-AxisValues))

(fn ConstructionScript)