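; PlayScreen_Shop is the shop play screen actor, which wires up its stations and shows the player's money.
; On BeginPlay it cross-links the meat printer, splicer, petri dish and phial managers, and hands the paper bag its order manager.
; It enables meat boxes from the game instance's AvailableMeat map and sets sort priorities for background, counter and register images.
; A looping timer refreshes the money text from the game instance.
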(event Custom|Update%20Money
  (bind _asmy_game_instance (Utilities|Casting|CastToMyGameInstance (Game|GetGameInstance)))
  (Rendering|Components|TextRender|SetText (Variables|Default|GetTextRender) (Utilities|Text|ToText(Integer) (Variables|/Game/Blueprints/MyGameInstance.MyGameInstance_C|Getcurrent_money _asmy_game_instance))))

(event EventBeginPlay
  (Utilities|FlowControl|Sequence
    (:then_0
      ;[0.4314 0.4314 0.4314] Set References
      (Variables|/Game/Blueprints/Machines/MeatPrinter.MeatPrinter_C|Setpetridish_manager_printer (Variables|Default|Getmeat_printer) (Variables|Default|Getpetri_manager_printer))
      (Variables|/Game/Blueprints/Managers/PetriDish_Manager_Printer.PetriDish_Manager_Printer_C|Setmeat_printer (Variables|Default|Getpetri_manager_printer) (Variables|Default|Getmeat_printer))
      (Variables|/Game/Blueprints/Machines/Splicer.Splicer_C|Setphial_manager (Variables|Default|Getsplicer) (Variables|Default|Getphial_manager))
      (Variables|/Game/Blueprints/Managers/Phial_Manager.Phial_Manager_C|Setsplicer (Variables|Default|Getphial_manager) (Variables|Default|Getsplicer))
      (Variables|/Game/Blueprints/Machines/Splicer.Splicer_C|Setpetridish_manager_splicer (Variables|Default|Getsplicer) (Variables|Default|Getpetri_manager_splicer))
      (Variables|/Game/Blueprints/Managers/PetriDish_Manager_Splicer.PetriDish_Manager_Splicer_C|Setsplicer (Variables|Default|Getpetri_manager_splicer) (Variables|Default|Getsplicer))
      (Variables|/Game/Blueprints/Managers/PetriDish_Manager_Splicer.PetriDish_Manager_Splicer_C|Setprinter_manager (Variables|Default|Getpetri_manager_splicer) (Variables|Default|Getpetri_manager_printer))
      (Variables|/Game/Blueprints/Managers/PetriDish_Manager_Printer.PetriDish_Manager_Printer_C|Setsplicer_manager (Variables|Default|Getpetri_manager_printer) (Variables|Default|Getpetri_manager_splicer))
      (Variables|/Game/Blueprints/Machines/PaperBag.PaperBag_C|Setorder_manager (Variables|Default|Getpaper_bag) (Variables|Default|Getorder_manager))
      (bind _asmy_game_instance (Utilities|Casting|CastToMyGameInstance (Game|GetGameInstance)))
      (for _array_element (Variables|Default|Getboxes)
        (Variables|/Game/Blueprints/Machines/PhialBox.PhialBox_C|Setenabled _array_element (and (.Value (Utilities|Map|Find (Variables|/Game/Blueprints/MyGameInstance.MyGameInstance_C|Getavailable_meat _asmy_game_instance) (Variables|/Game/Blueprints/Machines/PhialBox.PhialBox_C|Getmeat_type _array_element))) (.ReturnValue (Utilities|Map|Find (Variables|/Game/Blueprints/MyGameInstance.MyGameInstance_C|Getavailable_meat _asmy_game_instance) (Variables|/Game/Blueprints/Machines/PhialBox.PhialBox_C|Getmeat_type _array_element)))))
        (Default|UpdateImage _array_element)))
    (:then_1
      (Rendering|SetTranslucentSortPriority (Variables|Default|GetCounterImage) 1)
      (Rendering|SetTranslucentSortPriority (Variables|Default|GetBackgroundImage) 0)
      (Rendering|SetTranslucentSortPriority (Variables|Default|GetRegisterImage) 2))
    (:then_2
      (Utilities|Time|SetTimerbyFunctionName 0 "Update Money" 1.0 true))))

(fn ConstructionScript)